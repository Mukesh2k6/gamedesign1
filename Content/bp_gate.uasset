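; Gate Blueprint that swings its Doorframe open, both automatically shortly after BeginPlay and when an item-collection goal is met.
; CollectItem increments a counter, and a separate OpenDoorCheck event compares it to the maximum, calling OpenDoor through a DoOnce.
; OpenDoor plays a timeline that lerps the Doorframe's relative yaw to rotate it open.
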(event Custom|open%20door
  (bind _door_rotation (Timeline|open%20door%20animation Play)
    (:Update
      (Transformation|SetRelativeRotation (Variables|Default|Getdoorframe) (Math|Rotator|MakeRotator 0.0 0.0 (Math|Float|Lerp 0.0 1.2e+02 _door_rotation)) false false))))

(event Custom|collect%20item
  (Math|Integer|IncrementInt (Variables|Default|Getcurrent%20items%20collected)))

(event Custom|open%20door%20check
  (if (>= (Variables|Default|Getcurrent%20items%20collected) (Variables|Default|Getmax%20items%20collected))
    (Utilities|FlowControl|DoOnce false
      (:Completed
        (CallFunction|OpenDoor)))))

(event Custom|event%20begin%20play
  (Utilities|FlowControl|Delay 2.0)
  (CallFunction|OpenDoor))

(fn ConstructionScript)