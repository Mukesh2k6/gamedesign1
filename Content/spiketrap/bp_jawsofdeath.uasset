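; Jaws-of-death spike trap that snaps shut when its trigger box is overlapped.
; A timeline lerps the pitch of the mirrored left and right trap halves from 0 to 90 degrees, with no reopening logic.
; Overlapping either of two other boxes sends DeathMessage to the overlapping actor.
; All three overlap events call a player-check function, which returns no value to them.
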(event OnComponentBeginOverlap(triggerbox)
  (params (OverlappedComponent :type Primitive%20Component%20Object%20Reference) (OtherActor :type Actor%20Object%20Reference) (OtherComp :type Primitive%20Component%20Object%20Reference) (OtherBodyIndex :type Integer) (bFromSweep :type Boolean) (SweepResult :type Hit%20Result%20Structure%20%28by%20ref%29))
  (CallFunction|Checkifplayer OtherActor)
  (CallFunction|Startclose))

(event OnComponentBeginOverlap(Box2)
  (params (OverlappedComponent :type Primitive%20Component%20Object%20Reference) (OtherActor :type Actor%20Object%20Reference) (OtherComp :type Primitive%20Component%20Object%20Reference) (OtherBodyIndex :type Integer) (bFromSweep :type Boolean) (SweepResult :type Hit%20Result%20Structure%20%28by%20ref%29))
  (CallFunction|Checkifplayer OtherActor)
  (Class|BpiCharacter|Death(Message) OtherActor))

(event OnComponentBeginOverlap(Box1)
  (params (OverlappedComponent :type Primitive%20Component%20Object%20Reference) (OtherActor :type Actor%20Object%20Reference) (OtherComp :type Primitive%20Component%20Object%20Reference) (OtherBodyIndex :type Integer) (bFromSweep :type Boolean) (SweepResult :type Hit%20Result%20Structure%20%28by%20ref%29))
  (CallFunction|Checkifplayer OtherActor)
  (Class|BpiCharacter|Death(Message) OtherActor))

(event Custom|startclose
  (bind _closetrack (Timeline|close%20to%20jaws PlayFromStart)
    (:Update
      (Transformation|SetRelativeRotation (Variables|Default|GetrightTrap) (Math|Rotator|MakeRotator 0.0 (Math|Float|Lerp 0.0 9e+01 _closetrack) 0.0) false false)
      (Transformation|SetRelativeRotation (Variables|Default|GetleftTrap) (Math|Rotator|MakeRotator 0.0 (Math|Float|Lerp 0.0 9e+01 _closetrack) -1.8e+02) false false))))

(fn ConstructionScript)

(fn Checkifplayer
  (params (A :type Object%20Object%20Reference))
  (if (== A (Game|GetPlayerCharacter 0))
    (return)))